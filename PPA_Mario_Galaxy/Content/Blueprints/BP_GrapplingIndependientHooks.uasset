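; Physics-driven robot pawn with two independently controlled grappling hooks, one per arm.
; A camera-directed trace gates firing each tick; firing traces from a forearm socket, attaches a hook point to the hit component and shows a cable.
; While hooked, tick forces pull the physically animated body toward the hook and simulating objects toward the robot, scaled by inverse mass.
; Per-arm reel axes interpolate both pull forces between minimum and maximum.
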(event `self.ReceiveBeginPlay`
  (bind _minhookretractionforce (`self.minHookRetractionForce`))
  (bind _bone_name (`self.Bone Name`))
  (bind _minotherobjectretractionforce (`self.minOtherObjectRetractionForce`))
  (bind _physicalanimation (`self.PhysicalAnimation`))
  (bind _returnvalue (`|SpawnActorFromClass` "/Game/Blueprints/BP_HookPoint.BP_HookPoint_C" (`KismetMathLibrary.MakeTransform` (0.0 0.0 0.0)) "Undefined" "OverrideRootScale" null null))
  (set `self.RHookLocation` _returnvalue)
  (bind _returnvalue_2 (`|SpawnActorFromClass` "/Game/Blueprints/BP_HookPoint.BP_HookPoint_C" (`KismetMathLibrary.MakeTransform` (0.0 0.0 0.0)) "Undefined" "OverrideRootScale" null null))
  (set `self.LHookLocation` _returnvalue_2)
  (set `self.L_HookRetractionForce` _minhookretractionforce)
  (set `self.R_HookRetractionForce` _minhookretractionforce)
  (set `self.R_OtherObjectRetractionForce` _minotherobjectretractionforce)
  (set `self.L_OtherObjectRetractionForce` _minotherobjectretractionforce)
  (`PhysicalAnimationComponent.SetSkeletalMeshComponent` _physicalanimation (`self.Mesh`))
  (`PhysicalAnimationComponent.ApplyPhysicalAnimationSettingsBelow` _physicalanimation _bone_name (make `PhysicalAnimationData` false 1000.0 100.0 1000.0 100.0) false)
  (`SkeletalMeshComponent.SetAllBodiesBelowSimulatePhysics` (`self.Mesh`) _bone_name true false))

(event `InputAction|ShotLeftArm`
  (params (Key :type "Key Structure"))
  (:`Pressed`
    (if (`self.CanGrab`)
      (set `self.LeftFired` true)
      (set `self.SocketOrigin` "Robot-1-R-Forearm")
      (`self.SpawnHook` :!label _label)))
  (:`Released`
    (set `self.LHooked` false)
    (`SceneComponent.SetHiddenInGame` (`self.L_Cable`) true false)))

(event `UpdateSpringArm`
  ;[1 1 1] Spring Arm Update
  (`SceneComponent.K2_SetWorldLocation` (`self.SpringArm`) (+ (`SceneComponent.K2_GetComponentLocation` (`self.Mesh`)) (0.0 0.0 200.0)) false true))

(event `InputAction|ShotRightArm`
  (params (Key :type "Key Structure"))
  (:`Pressed`
    (if (`self.CanGrab`)
      (set `self.RightFired` true)
      (set `self.SocketOrigin` "Robot-1-L-Forearm")
      (goto _label)))
  (:`Released`
    (set `self.RHooked` false)
    (`SceneComponent.SetHiddenInGame` (`self.R_Cable`) true false)))

(event `InputAxis|LookUp`
  (params (AxisValue :type "Float (single-precision)"))
  ;[1 1 1] Camera Control
  (`self.AddControllerPitchInput` AxisValue))

(event `InputAxis|Turn`
  (params (AxisValue :type "Float (single-precision)"))
  ;[1 1 1] Camera Control
  (`self.AddControllerYawInput` AxisValue))

(event `InputAction|ReelIn`
  (params (Key :type "Key Structure")))

(event `InputAxis|ReelLeft`
  (params (AxisValue :type "Float (single-precision)"))
  (`/Engine/EditorBlueprintResources/StandardMacros.CompareFloat` AxisValue
    (:`>`
      (set `self.L_Reeling` false :!label _label_2))
    (:`==`
      (goto _label_2))
    (:`<`
      (set `self.L_Reeling` true)))
  (set `self.L_HookRetractionForce` (`KismetMathLibrary.Lerp` (`self.minHookRetractionForce`) (`self.MAXHookRetractionForce`) AxisValue))
  (set `self.L_OtherObjectRetractionForce` (`KismetMathLibrary.Lerp` (`self.minOtherObjectRetractionForce`) (`self.MAXOtherObjectRetractionForce`) AxisValue)))

(event `self.ReceiveTick`
  (params (DeltaSeconds :type "Float (single-precision)"))
  ;[1 1 1] Update
  (`|ExecutionSequence`
    (:`then_0`
      (`self.UpdateSpringArm`))
    (:`then_1`
      (`self.UpdateLaserAim`))
    (:`then_2`
      (`self.UpdateRightHook`))
    (:`then_3`
      (`self.UpdateLeftHook`))))

(event `InputAxis|ReelRight`
  (params (AxisValue :type "Float (single-precision)"))
  (`/Engine/EditorBlueprintResources/StandardMacros.CompareFloat` AxisValue
    (:`>`
      (set `self.R_Reeling` false :!label _label_3))
    (:`==`
      (goto _label_3))
    (:`<`
      (set `self.R_Reeling` true)))
  (set `self.R_HookRetractionForce` (`KismetMathLibrary.Lerp` (`self.minHookRetractionForce`) (`self.MAXHookRetractionForce`) AxisValue))
  (set `self.R_OtherObjectRetractionForce` (`KismetMathLibrary.Lerp` (`self.minOtherObjectRetractionForce`) (`self.MAXOtherObjectRetractionForce`) AxisValue)))

(fn `SpawnHook`
  (bind _lhooklocation (`self.LHookLocation`))
  (bind _r_cable (`self.R_Cable`))
  (bind _l_cable (`self.L_Cable`))
  (bind _rhooklocation (`self.RHookLocation`))
  (bind _camera (`self.Camera`))
  (bind (_outhit _returnvalue) (`KismetSystemLibrary.LineTraceSingleForObjects` (`SceneComponent.GetSocketLocation` (`self.Mesh`) (`self.SocketOrigin`)) (+ (`SceneComponent.K2_GetComponentLocation` _camera) (* (`SceneComponent.GetForwardVector` _camera) (`self.HookMaxDistance`))) (`|MakeArray` "ObjectTypeQuery1" "ObjectTypeQuery2" "ObjectTypeQuery4" "ObjectTypeQuery6" :!type "EObjectTypeQuery Enum")))
  (if _returnvalue
    (`|ExecutionSequence`
      (:`then_0`
        (if (`self.RightFired`)
          (set `self.RightFired` false)
          (set `self.RHooked` true)
          (`self.K2_DetachFromActor` "KeepRelative")
          (bind (_bblockinghit _binitialoverlap _time _distance _location _impactpoint _normal _impactnormal _physmat _hitactor _hitcomponent) (`GameplayStatics.BreakHitResult` _outhit))
          (`self.K2_SetActorLocation` _rhooklocation _location false false)
          (`self.K2_AttachToComponent` _rhooklocation _hitcomponent "None" "KeepWorld" "KeepRelative" "KeepRelative" true)
          (`SceneComponent.SetHiddenInGame` _r_cable false false)
          (set `self.RGrappledComponent` _hitcomponent)
          (`CableComponent.SetAttachEndTo` _r_cable (`self.RHookLocation`) "None" "None")))
      (:`then_1`
        (if (`self.LeftFired`)
          (set `self.LeftFired` false)
          (set `self.LHooked` true)
          (`self.K2_DetachFromActor` _lhooklocation "KeepRelative" "KeepRelative" "KeepRelative")
          (`self.K2_SetActorLocation` _lhooklocation _location false false)
          (`self.K2_AttachToComponent` _lhooklocation _hitcomponent "None" "KeepWorld" "KeepRelative" "KeepRelative" true)
          (`SceneComponent.SetHiddenInGame` _l_cable false false)
          (set `self.LGrappledComponent` _hitcomponent)
          (`CableComponent.SetAttachEndTo` _l_cable (`self.LHookLocation`) "None" "None"))))))

(fn `UpdateLaserAim`
  (bind _camera (`self.Camera`))
  (bind (_outhit _returnvalue) (`KismetSystemLibrary.LineTraceSingleForObjects` :`Start` (`SceneComponent.GetSocketLocation` (`self.Mesh`) "Robot-1-Head") :`End` (+ (`SceneComponent.K2_GetComponentLocation` _camera) (* (`SceneComponent.GetForwardVector` _camera) (`self.HookMaxDistance`))) :`ObjectTypes` (`|MakeArray` "ObjectTypeQuery1" "ObjectTypeQuery2" "ObjectTypeQuery6" "ObjectTypeQuery4" :!type "EObjectTypeQuery Enum") :`bTraceComplex` true :`DrawTime` 0.0))
  (if _returnvalue
    (set `self.CanGrab` true)
    (`KismetSystemLibrary.DrawDebugSphere` (`.Location` (`GameplayStatics.BreakHitResult` _outhit)) 20.0 20 (struct :`R` 1.0 :`B` 0.023573 :`A` 1.0) 0.0 1.0)
    (else
      (set `self.CanGrab` false))))

(fn `UpdateLeftHook`
  (bind _lgrappledcomponent (`self.LGrappledComponent`))
  (if (`self.LHooked`)
    (if (`SceneComponent.IsSimulatingPhysics` _lgrappledcomponent "None")
      (`PrimitiveComponent.AddForce` _lgrappledcomponent (* (`KismetMathLibrary.Normal` (- (`SceneComponent.K2_GetComponentLocation` (`self.Mesh`)) (`self.K2_GetActorLocation` (`self.LHookLocation`)))) (/ (`self.L_OtherObjectRetractionForce`) (`PrimitiveComponent.GetMass` _lgrappledcomponent))) "None" true))
    (`SkeletalMeshComponent.AddForceToAllBodiesBelow` (`self.Mesh`) (* (`KismetMathLibrary.Normal` (- (`self.K2_GetActorLocation` (`self.LHookLocation`)) (`SceneComponent.K2_GetComponentLocation` (`self.Mesh`)))) (`self.L_HookRetractionForce`)) "Robot-1-L-Forearm" true true)))

(fn `UpdateRightHook`
  (bind _rgrappledcomponent (`self.RGrappledComponent`))
  (if (`self.RHooked`)
    (if (`SceneComponent.IsSimulatingPhysics` _rgrappledcomponent "None")
      (`PrimitiveComponent.AddForce` _rgrappledcomponent (* (`KismetMathLibrary.Normal` (- (`SceneComponent.K2_GetComponentLocation` (`self.Mesh`)) (`self.K2_GetActorLocation` (`self.RHookLocation`)))) (/ (`self.R_OtherObjectRetractionForce`) (`PrimitiveComponent.GetMass` _rgrappledcomponent))) "None" true))
    (`SkeletalMeshComponent.AddForceToAllBodiesBelow` (`self.Mesh`) (* (`KismetMathLibrary.Normal` (- (`self.K2_GetActorLocation` (`self.RHookLocation`)) (`SceneComponent.K2_GetComponentLocation` (`self.Mesh`)))) (`self.R_HookRetractionForce`)) "Robot-1-R-Forearm" true true)))

(fn `UserConstructionScript`)