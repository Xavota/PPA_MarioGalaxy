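; BP_Meteorite is a destructible meteorite whose pieces are pushed by a radial force when it fractures.
; The construction script lowers its mass scale, and the fracture event flags it destroyed and applies an acceleration-based radial force, using its bounds radius for both radius and strength.
; A disconnected gravity-style pull on overlapping physics bodies, with debug print and lines, never runs and has a zero force multiplier.
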(event `self.ReceiveTick`
  (params (DeltaSeconds :type "Float (single-precision)")))

(event `self.Destructible.OnComponentFracture`
  (params (HitPoint :type "Vector Structure (by ref)") (HitDirection :type "Vector Structure (by ref)"))
  (bind _destructible (`self.Destructible`))
  (bind (_origin _boxextent _sphereradius) (`KismetSystemLibrary.GetComponentBounds` _destructible))
  (set `self.IsDestroyed` true)
  (`PrimitiveComponent.AddRadialForce` _destructible (`SceneComponent.K2_GetComponentLocation` _destructible) _sphereradius _sphereradius "RIF_Constant" true))

(fn `UserConstructionScript`
  (`PrimitiveComponent.SetMassScale` (`self.Destructible`) "None" 0.1))