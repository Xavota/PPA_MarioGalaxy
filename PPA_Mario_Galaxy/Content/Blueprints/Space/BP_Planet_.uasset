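; Planet actor that acts as a gravity source, pulling nearby physics objects toward its center of mass.
; The construction script sizes the GravityRange sphere from GravityRadius.
; Each tick, every overlapping simulating component except the planet receives a force of its mass times Gravity, with no distance falloff.
; A debug line is drawn from the planet to each affected component.
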(event `self.ReceiveTick`
  (params (DeltaSeconds :type "Float (single-precision)"))
  (bind _returnvalue (`PrimitiveComponent.GetCenterOfMass` (`self.Planet`) "None"))
  (for _array_element (`PrimitiveComponent.GetOverlappingComponents` (`self.GravityRange`))
    (if (and (`SceneComponent.IsSimulatingPhysics` _array_element "None") (!= _array_element (`self.Planet`)))
      (bind _returnvalue_2 (`PrimitiveComponent.GetCenterOfMass` _array_element "None"))
      (`PrimitiveComponent.AddForceAtLocation` _array_element (* (`KismetMathLibrary.Normal` (- _returnvalue _returnvalue_2)) (* (`PrimitiveComponent.GetMass` _array_element) (`self.Gravity`))) _returnvalue_2 "None")
      (`KismetSystemLibrary.DrawDebugLine` _returnvalue _returnvalue_2 (struct :`R` 1.0 :`B` 0.201579 :`A` 1.0) 0.0 1.0))))

(fn `UserConstructionScript`
  (`SphereComponent.SetSphereRadius` (`self.GravityRange`) (`self.GravityRadius`) true))