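; BP_Planet_ is a planet or moon with its own gravity field, given a random mesh and scaled at construction.
; Each tick, non-player physics bodies inside GravityRange are pulled toward its center, with debug lines, while player overlaps trigger a surface trace that sets pawn roll.
; Entering or leaving the range switches the player's NinjaCharacter collision-based gravity.
; OverlappingComponentIsPlayer's True exit means non-player, and enemy-spawning PoblatePlanet is never run.
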(event `self.ReceiveBeginPlay`
  (set `self.PlayerPawnClass` (`GameplayStatics.GetObjectClass` (`GameplayStatics.GetPlayerPawn` 0)))
  (if (`self.isPlanet`)
    _))

(event `self.ReceiveTick`
  (params (DeltaSeconds :type "Float (single-precision)"))
  (bind _returnvalue (`PrimitiveComponent.GetCenterOfMass` (`self.Astro`) "None"))
  (for _array_element (`PrimitiveComponent.GetOverlappingComponents` (`self.GravityRange`))
    (`self.OverlappingComponentIsPlayer` _array_element
      (:`True`
        (`self.OverlappingComponentIsSImulatingPhysics` _array_element
          (:`True`
            (bind _returnvalue_2 (`PrimitiveComponent.GetCenterOfMass` _array_element "None"))
            (`PrimitiveComponent.AddForceAtLocation` _array_element (* (`KismetMathLibrary.Normal` (- _returnvalue _returnvalue_2)) (* (`PrimitiveComponent.GetMass` _array_element) (`self.Gravity`))) _returnvalue_2 "None")
            (`KismetSystemLibrary.DrawDebugLine` _returnvalue _returnvalue_2 (struct :`R` 1.0 :`B` 0.201579 :`A` 1.0) 0.0 1.0))))
      (:`False`
        (bind _outhit (`KismetSystemLibrary.LineTraceSingleForObjects` :`Start` (`PrimitiveComponent.GetCenterOfMass` _array_element "None") :`End` (`PrimitiveComponent.GetCenterOfMass` (`self.Astro`) "None") :`ObjectTypes` (`self.Object Types`) :`bTraceComplex` true :`DrawDebugType` "ForOneFrame"))
        (if (> (`.Distance` (`GameplayStatics.BreakHitResult` _outhit)) 50.0)
          (bind _returnvalue_roll (`KismetMathLibrary.BreakRotator` (`KismetMathLibrary.Conv_VectorToRotator` (`.Normal` (`GameplayStatics.BreakHitResult` _outhit)))))
          (`self.K2_SetActorRotation` (`GameplayStatics.GetPlayerPawn` 0) (`KismetMathLibrary.MakeRotator` _returnvalue_roll) false))))))

(event `self.GravityRange.OnComponentBeginOverlap`
  (params (OverlappedComponent :type "PrimitiveComponent Object Reference") (OtherActor :type "Actor Object Reference") (OtherComp :type "PrimitiveComponent Object Reference") (OtherBodyIndex :type Integer) (bFromSweep :type Boolean) (SweepResult :type "HitResult Structure (by ref)"))
  (if (== (`GameplayStatics.GetObjectClass` OtherActor) (`self.PlayerPawnClass`))
    (`PrimitiveComponent.SetEnableGravity` OtherComp true)
    (bind _asninja_character (cast `NinjaCharacter` OtherActor))
    (bind _asninja_character_movement_component (cast `NinjaCharacterMovementComponent` (`Character.CharacterMovement` _asninja_character)))
    (`NinjaCharacterMovementComponent.SetCollisionGravityDirection` _asninja_character_movement_component (`self.CenterOfMass`))
    (set `CharacterMovementComponent.GravityScale` (/ (`self.Gravity`) 100.0) _asninja_character_movement_component)))

(event `self.GravityRange.OnComponentEndOverlap`
  (params (OverlappedComponent :type "PrimitiveComponent Object Reference") (OtherActor :type "Actor Object Reference") (OtherComp :type "PrimitiveComponent Object Reference") (OtherBodyIndex :type Integer))
  (if (== (`GameplayStatics.GetObjectClass` OtherActor) (`self.PlayerPawnClass`))
    (`PrimitiveComponent.SetEnableGravity` OtherComp false)
    (bind _asninja_character (cast `NinjaCharacter` OtherActor))
    (bind _asninja_character_movement_component (cast `NinjaCharacterMovementComponent` (`Character.CharacterMovement` _asninja_character)))
    (`NinjaCharacterMovementComponent.SetCollisionGravityDirection` _asninja_character_movement_component null)))

(fn `PoblatePlanet`
  (for _ (range 10)
    (bind _outhit (`KismetSystemLibrary.LineTraceSingleForObjects` :`Start` (* (`KismetMathLibrary.RandomUnitVector`) (`SphereComponent.GetScaledSphereRadius` (`self.GravityRange`))) :`End` (`SceneComponent.K2_GetComponentLocation` (`self.Astro`)) :`ObjectTypes` (`|MakeArray` "ObjectTypeQuery2" :!type "EObjectTypeQuery Enum") :`DrawDebugType` "ForDuration" :`bIgnoreSelf` false :`DrawTime` 1.0))
    (bind (_bblockinghit _binitialoverlap _time _distance _location _impactpoint _normal _impactnormal) (`GameplayStatics.BreakHitResult` _outhit))
    (`|SpawnActorFromClass` "/Game/Blueprint/Enemy_BP.Enemy_BP_C" (`KismetMathLibrary.MakeTransform` _impactpoint (`KismetMathLibrary.Conv_VectorToRotator` _impactnormal) (10.0 10.0 10.0)) "Undefined" "OverrideRootScale" null null)))

(fn `UserConstructionScript`
  (switch `/Game/Maiiki/Blueprints/AstroTypes` (`self.AstroType`)
    (:`NewEnumerator0`
      (bind _returnvalue (`StaticMeshComponent.SetStaticMesh` (`self.Astro`) (`KismetArrayLibrary.Array_Random` (`self.Exoplanets`))))
      (set `self.isPlanet` _returnvalue))
    (:`NewEnumerator1`
      (`StaticMeshComponent.SetStaticMesh` (`self.Astro`) (`KismetArrayLibrary.Array_Random` (`self.Moons`)))))
  (`SceneComponent.SetWorldScale3D` (`self.Astro`) (`KismetMathLibrary.Conv_DoubleToVector` (`self.Scale`)))
  (`SphereComponent.SetSphereRadius` (`self.GravityRange`) (/ (`.SphereRadius` (`KismetSystemLibrary.GetComponentBounds` (`self.Astro`))) 35.0) true))