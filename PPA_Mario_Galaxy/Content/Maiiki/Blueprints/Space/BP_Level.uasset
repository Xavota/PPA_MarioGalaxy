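; BP_Level builds a bounded space level filled with debris, planets and meteorites.
; On BeginPlay it spawns set quantities of each at random directions and distances around the world origin, with random rotation and scale, turning gravity off on debris.
; The LevelLimits sphere, sized from LimitRadius at construction, turns back exiting physics-simulating components with a velocity-change impulse that slightly exceeds and opposes their velocity.
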(event `self.ReceiveBeginPlay`
  (`self.SpawnDebris`))

(event `self.LevelLimits.OnComponentEndOverlap`
  (params (OverlappedComponent :type "PrimitiveComponent Object Reference") (OtherActor :type "Actor Object Reference") (OtherComp :type "PrimitiveComponent Object Reference") (OtherBodyIndex :type Integer))
  (if (`SceneComponent.IsSimulatingPhysics` OtherComp "None")
    (bind _returnvalue (`PrimitiveComponent.GetPhysicsLinearVelocity` OtherComp "None"))
    (`PrimitiveComponent.AddImpulse` OtherComp (* (`KismetMathLibrary.NegateVector` _returnvalue) 1.1) "None" true)))

(fn `SpawnDebris`
  (bind _returnvalue (`KismetMathLibrary.RandomFloatInRange` 5.0 20.0))
  (bind _returnvalue_2 (`KismetMathLibrary.RandomFloatInRange` 50.0 200.0))
  (bind _returnvalue_3 (`KismetMathLibrary.RandomFloatInRange` 20.0 30.0))
  (for _ (range 1 (+ (`self.DebrisQtt`) 1))
    (bind _returnvalue_4 (`|SpawnActorFromClass` "/Game/Maiiki/Blueprints/Space/BP_Debri.BP_Debri_C" (`KismetMathLibrary.MakeTransform` (* (`KismetMathLibrary.RandomUnitVector`) (`KismetMathLibrary.RandomFloatInRange` 5000.0 (- (`self.LimitRadius`) 100.0))) (`KismetMathLibrary.RandomRotator` true) (`KismetMathLibrary.MakeVector` _returnvalue _returnvalue 0.1)) "AdjustIfPossibleButAlwaysSpawn" "OverrideRootScale" null null))
    (`PrimitiveComponent.SetEnableGravity` (`/Game/Maiiki/Blueprints/Space/BP_Debri.StaticMeshComponent0` _returnvalue_4) false))
  (for _ (range 1 (+ (`self.PlanetsQtt`) 1))
    (`|SpawnActorFromClass` "/Game/Maiiki/Blueprints/Space/BP_Planet_.BP_Planet__C" (`KismetMathLibrary.MakeTransform` (* (`KismetMathLibrary.RandomUnitVector`) (`KismetMathLibrary.RandomFloatInRange` 15000.0 (- (`self.LimitRadius`) 100.0))) (`KismetMathLibrary.RandomRotator` true) (`KismetMathLibrary.MakeVector` _returnvalue_2 _returnvalue_2 _returnvalue_2)) "AdjustIfPossibleButAlwaysSpawn" "OverrideRootScale" null null))
  (for _ (range 1 (+ (`self.MeteorQtt`) 1))
    (`|SpawnActorFromClass` "/Game/Maiiki/Blueprints/Space/BP_Meteorite.BP_Meteorite_C" (`KismetMathLibrary.MakeTransform` (* (`KismetMathLibrary.RandomUnitVector`) (`KismetMathLibrary.RandomFloatInRange` 1000.0 (- (`self.LimitRadius`) 100.0))) (`KismetMathLibrary.RandomRotator` true) (`KismetMathLibrary.MakeVector` _returnvalue_3 _returnvalue_3 _returnvalue_3)) "AdjustIfPossibleButAlwaysSpawn" "OverrideRootScale" null null)))

(fn `UserConstructionScript`
  (`SphereComponent.SetSphereRadius` (`self.LevelLimits`) (`self.LimitRadius`) true))