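; Celestial body (planet or moon) with its own gravity field, randomizing its mesh by type and sizing the GravityRange sphere to it.
; Each tick pulls overlapping non-player physics bodies toward its center with mass-scaled force.
; NinjaCharacters in range get collision gravity aimed at a spawned CenterOfMass actor that follows the body; leaving weakens the player's gravity.
; On BeginPlay, planets scatter MaiikiCoins over their surface using random inward line traces.
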(event `self.ReceiveTick`
  (params (DeltaSeconds :type "Float (single-precision)"))
  (bind _returnvalue (`PrimitiveComponent.GetCenterOfMass` (`self.Astro`) "None"))
  (`|ExecutionSequence`
    (:`then_0`
      (for _array_element (`PrimitiveComponent.GetOverlappingComponents` (`self.GravityRange`))
        (`self.OverlappingComponentIsPlayer` _array_element
          (:`True`
            (`self.OverlappingComponentIsSImulatingPhysics` _array_element
              (:`True`
                (bind _returnvalue_2 (`PrimitiveComponent.GetCenterOfMass` _array_element "None"))
                (`PrimitiveComponent.AddForceAtLocation` _array_element (* (`KismetMathLibrary.Normal` (- _returnvalue _returnvalue_2)) (* (`PrimitiveComponent.GetMass` _array_element) (`self.Gravity`))) _returnvalue_2 "None")
                (`KismetSystemLibrary.DrawDebugLine` _returnvalue _returnvalue_2 (struct :`R` 1.0 :`B` 0.201579 :`A` 1.0) 0.0 1.0)))))))
    (:`then_1`
      (`self.UpdateCenterOfMass`))))

(event `self.ReceiveBeginPlay`
  (bind _returnvalue (`KismetSystemLibrary.GetDisplayName` self))
  (`|ExecutionSequence`
    (:`then_0`
      (set `self.PlayerPawnClass` (`GameplayStatics.GetObjectClass` (`GameplayStatics.GetPlayerPawn` 0)))
      (if (`self.isPlanet`)
        (`self.PoblatePlanet`)))
    (:`then_1`
      (`self.UpdateCenterOfMass`))
    (:`then_2`
      (`KismetSystemLibrary.PrintString` _returnvalue true true (struct :`R` 1.0 :`B` 0.053333 :`A` 1.0) 20.0)
      (for _array_element (`self.GetOverlappingActors` null)
        (if (`KismetStringLibrary.EqualEqual_StrStr` _returnvalue "BP_Planet_2")
          (cast `/Game/Maiiki/Blueprints/MaiikiCoin_BP` _array_element
            (:`CastFailed`
              (`KismetSystemLibrary.PrintString` (`KismetStringLibrary.Concat_StrStr` "    " (`KismetSystemLibrary.GetDisplayName` _array_element)) true true (struct :`G` 0.66 :`B` 1.0 :`A` 1.0) 20.0))))
        (bind _asninja_character (cast `NinjaCharacter` _array_element))
        (bind _asninja_character_movement_component (cast `NinjaCharacterMovementComponent` (`Character.CharacterMovement` _asninja_character)))
        (`NinjaCharacterMovementComponent.SetCollisionGravityDirection` _asninja_character_movement_component (`self.CenterOfMass`))
        (set `CharacterMovementComponent.GravityScale` (/ (`self.Gravity`) 100.0) _asninja_character_movement_component)))))

(event `self.GravityRange.OnComponentBeginOverlap`
  (params (OverlappedComponent :type "PrimitiveComponent Object Reference") (OtherActor :type "Actor Object Reference") (OtherComp :type "PrimitiveComponent Object Reference") (OtherBodyIndex :type Integer) (bFromSweep :type Boolean) (SweepResult :type "HitResult Structure (by ref)"))
  (`PrimitiveComponent.SetEnableGravity` OtherComp true)
  (bind _asninja_character (cast `NinjaCharacter` OtherActor))
  (bind _asninja_character_movement_component (cast `NinjaCharacterMovementComponent` (`Character.CharacterMovement` _asninja_character)))
  (`NinjaCharacterMovementComponent.SetCollisionGravityDirection` _asninja_character_movement_component (`self.CenterOfMass`))
  (set `CharacterMovementComponent.GravityScale` (/ (`self.Gravity`) 100.0) _asninja_character_movement_component))

(event `self.GravityRange.OnComponentEndOverlap`
  (params (OverlappedComponent :type "PrimitiveComponent Object Reference") (OtherActor :type "Actor Object Reference") (OtherComp :type "PrimitiveComponent Object Reference") (OtherBodyIndex :type Integer))
  (if (== (`GameplayStatics.GetObjectClass` OtherActor) (`self.PlayerPawnClass`))
    (`PrimitiveComponent.SetEnableGravity` OtherComp false)
    (bind _asninja_character (cast `NinjaCharacter` OtherActor))
    (bind _asninja_character_movement_component (cast `NinjaCharacterMovementComponent` (`Character.CharacterMovement` _asninja_character)))
    (`NinjaCharacterMovementComponent.SetCollisionGravityDirection` _asninja_character_movement_component null)
    (set `CharacterMovementComponent.GravityScale` (/ (`CharacterMovementComponent.GravityScale` _asninja_character_movement_component) 1000.0) _asninja_character_movement_component)))

(fn `PoblatePlanet`
  (bind _returnvalue (* (`KismetMathLibrary.RandomUnitVector`) (`SphereComponent.GetScaledSphereRadius` (`self.GravityRange`))))
  (for _ (range (+ (`KismetMathLibrary.RandomInteger` 100) 1))
    (bind _outhit (`KismetSystemLibrary.LineTraceSingleForObjects` :`Start` _returnvalue :`End` (`SceneComponent.K2_GetComponentLocation` (`self.Astro`)) :`ObjectTypes` (`|MakeArray` "ObjectTypeQuery2" :!type "EObjectTypeQuery Enum") :`DrawDebugType` "ForDuration" :`bIgnoreSelf` false :`DrawTime` 1.0))
    (bind (_bblockinghit _binitialoverlap _time _distance _location _impactpoint _normal _impactnormal) (`GameplayStatics.BreakHitResult` _outhit))
    (`|SpawnActorFromClass` "/Game/Maiiki/Blueprints/MaiikiCoin_BP.MaiikiCoin_BP_C" (`KismetMathLibrary.MakeTransform` (- _location (* (`KismetMathLibrary.Normal` _returnvalue) 50.0)) (`KismetMathLibrary.Conv_VectorToRotator` _impactnormal)) "Undefined" "OverrideRootScale" null null)))

(fn `UpdateCenterOfMass`
  (bind _returnvalue (`self.K2_GetActorLocation`))
  (bind _centerofmass (`self.CenterOfMass`))
  (bind _sphere (`/Game/Mara/Blueprints/CenterOfMass_BP.Sphere` _centerofmass))
  (`/Engine/EditorBlueprintResources/StandardMacros.IsValid` _centerofmass
    (:`Is Valid`
      (`SceneComponent.SetMobility` _sphere "Movable")
      (`self.K2_SetActorLocation` _centerofmass _returnvalue false false)
      (`SceneComponent.SetMobility` _sphere "Static"))
    (:`Is Not Valid`
      (bind _returnvalue_2 (`|SpawnActorFromClass` "/Game/Mara/Blueprints/CenterOfMass_BP.CenterOfMass_BP_C" (`KismetMathLibrary.MakeTransform` _returnvalue) "Undefined" "OverrideRootScale" null null))
      (set `self.CenterOfMass` _returnvalue_2))))

(fn `UserConstructionScript`
  (switch `/Game/Maiiki/Blueprints/AstroTypes` (`self.AstroType`)
    (:`NewEnumerator0`
      (bind _returnvalue (`StaticMeshComponent.SetStaticMesh` (`self.Astro`) (`KismetArrayLibrary.Array_Random` (`self.Exoplanets`))))
      (set `self.isPlanet` _returnvalue))
    (:`NewEnumerator1`
      (`StaticMeshComponent.SetStaticMesh` (`self.Astro`) (`KismetArrayLibrary.Array_Random` (`self.Moons`)))))
  (`SceneComponent.SetWorldScale3D` (`self.Astro`) (`KismetMathLibrary.Conv_DoubleToVector` (`self.Scale`)))
  (`SphereComponent.SetSphereRadius` (`self.GravityRange`) (/ (`.SphereRadius` (`KismetSystemLibrary.GetComponentBounds` (`self.Astro`))) 35.0) true))