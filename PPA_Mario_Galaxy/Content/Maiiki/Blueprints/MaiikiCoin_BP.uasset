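; MaiikiCoin_BP is a coin pickup that homes in on the player once the player comes within its attraction range.
; The AtractionRange overlap stores the player's overlapping component as a target, and Tick moves the Coin toward it at a fixed Speed per frame, without delta-time scaling.
; Touching the Collider spawns a spark effect and destroys the coin.
; A helper macro identifies the player by matching class against player pawn 0.
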(event `self.ReceiveTick`
  (params (DeltaSeconds :type "Float (single-precision)"))
  (bind _coin (`self.Coin`))
  (`/Engine/EditorBlueprintResources/StandardMacros.IsValid` (`self.TargetComponent`)
    (:`Is Valid`
      (`SceneComponent.K2_AddWorldOffset` _coin (* (`KismetMathLibrary.Normal` (- (`SceneComponent.K2_GetComponentLocation` (`self.TargetComponent`)) (`SceneComponent.K2_GetComponentLocation` _coin))) (`self.Speed`)) false false))))

(event `self.Collider.OnComponentBeginOverlap`
  (params (OverlappedComponent :type "PrimitiveComponent Object Reference") (OtherActor :type "Actor Object Reference") (OtherComp :type "PrimitiveComponent Object Reference") (OtherBodyIndex :type Integer) (bFromSweep :type Boolean) (SweepResult :type "HitResult Structure (by ref)"))
  (`self.ActorClassIsEqualToPlayetClass` OtherActor
    (:`True`
      (`GameplayStatics.SpawnEmitterAtLocation` "/Game/CelebrationVFXPack/Particles/P_explosion_sparks.P_explosion_sparks" (`SceneComponent.K2_GetComponentLocation` (`self.Coin`)))
      (`self.K2_DestroyActor`))))

(event `self.AtractionRange.OnComponentBeginOverlap`
  (params (OverlappedComponent :type "PrimitiveComponent Object Reference") (OtherActor :type "Actor Object Reference") (OtherComp :type "PrimitiveComponent Object Reference") (OtherBodyIndex :type Integer) (bFromSweep :type Boolean) (SweepResult :type "HitResult Structure (by ref)"))
  (`self.ActorClassIsEqualToPlayetClass` (`ActorComponent.GetOwner` OtherComp)
    (:`True`
      (set `self.TargetComponent` OtherComp))))

(fn `UserConstructionScript`)