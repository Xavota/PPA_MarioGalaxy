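; AI controller for the alien that runs the Alien_BT behavior tree on possession and tracks the player through AI Perception.
; Sensing a Player-tagged actor cancels the forget timer and writes HasLineOfSight and Enemy to the Blackboard.
; Any other perception update, including non-player actors, starts a LineOfSightTimer-length delay before clearing both keys.
; Each update also prints a "SEE" debug message.
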(event `self.ReceivePossess`
  (params (PossessedPawn :type "Pawn Object Reference"))
  (`self.RunBehaviorTree` "/Game/Mara/Blueprints/IA/Alien_BT.Alien_BT"))

(event `self.AIPerception.OnTargetPerceptionUpdated`
  (params (Actor :type "Actor Object Reference") (Stimulus :type "AIStimulus Structure"))
  (bind _blackboard (`self.Blackboard`))
  (`KismetSystemLibrary.PrintString` "SEE" true true (struct :`R` 1.0 :`B` 0.223794 :`A` 1.0))
  (if (and (`self.ActorHasTag` Actor "Player") (`.bSuccessfullySensed` (break `AIStimulus` Stimulus)))
    (`KismetSystemLibrary.K2_ClearAndInvalidateTimerHandle` (`self.EventTimer`))
    (`BlackboardComponent.SetValueAsBool` _blackboard (`self.HasLineOfSight`) true)
    (`BlackboardComponent.SetValueAsObject` _blackboard (`self.Enemy`) Actor)
    (else
      (bind _returnvalue (`KismetSystemLibrary.K2_SetTimerDelegate` (delegate `StartEnemyTimer`) (`self.LineOfSightTimer`)))
      (set `self.EventTimer` _returnvalue))))

(event `StartEnemyTimer`
  (bind _blackboard (`self.Blackboard`))
  (`BlackboardComponent.SetValueAsBool` _blackboard (`self.HasLineOfSight`) false)
  (`BlackboardComponent.SetValueAsObject` _blackboard (`self.Enemy`) null))

(fn `UserConstructionScript`)